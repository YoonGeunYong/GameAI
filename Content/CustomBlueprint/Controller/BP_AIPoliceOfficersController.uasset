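; AI controller for police officers that runs the BT_Police behavior tree and feeds it sightings of the thief.
; Perception updates pass through HandleSightSense, which reacts only to sight stimuli from BP_Thief actors.
; A successful sighting sets the TargetThief blackboard key; losing sight clears it and stores the stimulus location as ThiefLastPosition.
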(event OnTargetPerceptionUpdated(AIPerception)
  (params (Actor :type Actor%20Object%20Reference) (Stimulus :type AI%20Stimulus%20Structure))
  (CallFunction|HandleSightSense Actor Stimulus))

(event EventBeginPlay
  (AI|RunBehaviorTree "/Game/CustomBlueprint/AI_Related/BT_Police.BT_Police"))

(event EventTick
  (params (DeltaSeconds :type Float%20%28single-precision%29)))

(fn ConstructionScript)

(fn HandleSightSense
  (params (Actor :type Actor%20Object%20Reference) (Stimulus :type AI%20Stimulus%20Structure))
  (bind _returnvalue (Class|AIPerceptionSystem|GetSenseClassforStimulus Stimulus))
  (if (== _returnvalue "/Script/AIModule.AISense_Sight")
    (if (== Actor (.AsBP%20Thief (Utilities|Casting|CastToBP_Thief Actor)))
      (AI|Components|Blackboard|SetValueasObject (Variables|Default|GetBlackboard) (Utilities|Name|MakeLiteralName "TargetThief") (Utilities|SelectObject (.AsBP%20Thief (Utilities|Casting|CastToBP_Thief Actor)) 0 (.bsuccessfullysensed Stimulus)))
      (if (not (.bsuccessfullysensed Stimulus))
        (AI|Components|Blackboard|SetValueasVector (Variables|Default|GetBlackboard) (Utilities|Name|MakeLiteralName "ThiefLastPosition") (.stimuluslocation Stimulus)))
      (else
        (return)))
    (else
      (return))))